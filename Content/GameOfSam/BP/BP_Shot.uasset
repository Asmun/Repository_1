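; BP_Shot is a projectile fired in connection with the player character BP_Dude, using a Box collider and ProjectileMovement.
; It destroys itself when the Box hits something, and on destruction notifies the player's BP_Dude through ShotDestroyed.
; A ShootDown event sends it downward at max speed, rotates the Box, and offsets it by the player's facing and GunDownOffset, with a debug print of Facing.
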(event `self.Box.OnComponentHit`
  (params (HitComponent :type "PrimitiveComponent Object Reference") (OtherActor :type "Actor Object Reference") (OtherComp :type "PrimitiveComponent Object Reference") (NormalImpulse :type "Vector Structure") (Hit :type "HitResult Structure (by ref)"))
  (`self.K2_DestroyActor`))

(event `self.ReceiveDestroyed`
  (bind _asbp_dude (cast `/Game/GameOfSam/BP/BP_Dude` (`GameplayStatics.GetPlayerCharacter` 0)))
  (`/Game/GameOfSam/BP/BP_Dude.ShotDestroyed` _asbp_dude))

(event `ShootDown`
  (bind _box (`self.Box`))
  (`ProjectileMovementComponent.SetVelocityInLocalSpace` (`self.ProjectileMovement`) (`KismetMathLibrary.MakeVector` 0.0 0.0 (* (`MovementComponent.GetMaxSpeed` (`self.ProjectileMovement`)) -1.0)))
  (`SceneComponent.K2_SetRelativeRotation` _box (struct :`Pitch` -90.0) false false)
  (bind _asbp_dude (cast `/Game/GameOfSam/BP/BP_Dude` (`GameplayStatics.GetPlayerCharacter` 0)))
  (bind _facing (`/Game/GameOfSam/BP/BP_Dude.Facing` _asbp_dude))
  (`KismetSystemLibrary.PrintString` (`KismetStringLibrary.Conv_IntToString` _facing))
  (`SceneComponent.K2_AddRelativeLocation` _box (`KismetMathLibrary.MakeVector` (`KismetMathLibrary.Conv_IntToDouble` (* _facing (`self.GunDownOffset`))) 0.0 -6.0) false false))

(fn `UserConstructionScript`)