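; BP_Dude is the player's 2D side-scrolling character, with run, jump, shoot, health and a HUD.
; A state enum picks the flipbook each tick, while horizontal velocity sets facing.
; Shooting is capped by delay and live-shot count and refires while held; airborne shots fire downward with recoil.
; Damage (or debug key 1) knocks back and locks input until landing, which also resets Dead; the blink is unfinished, leaving the sprite hidden.
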(event `Key|One`
  (params (Key :type "Key Structure"))
  ;[1 0 0] Taking Damage
  (:`Pressed`
    (`self.DisableInput` (`GameplayStatics.GetPlayerController` 0) :!label _label)
    (bind _output_get (set `self.HealthCurrent` (- (`self.HealthCurrent`) (`KismetMathLibrary.FTrunc` (stale `Damage System` DamageIn)))))
    (set `MovementComponent.Velocity` (0.0 0.0 0.0) (`self.CharacterMovement`))
    (`self.LaunchCharacter` (`KismetMathLibrary.MakeVector` (`KismetMathLibrary.Conv_IntToDouble` (* (`self.Facing`) (`self.Knockback`))) 0.0 300.0))
    (if (<= _output_get 0)
      (set `self.CharacterState` "NewEnumerator5")
      (`self.DisableInput` (`GameplayStatics.GetPlayerController` 0))
      (`self.UpdateAnimation`)
      (else
        (bind _returnvalue (`KismetSystemLibrary.K2_SetTimerDelegate` (delegate `Blink`) 0.2 true))
        (`SceneComponent.SetHiddenInGame` (`self.Sprite`) true false)))))

(event `Damage System`
  (params (DamageIn :type "Float (double-precision)"))
  ;[1 0 0] Taking Damage
  (goto _label))

(event `Blink`
  ;[1 0 0] Taking Damage
)

(event `self.ReceiveBeginPlay`
  ;[1 1 1] Initializing
  (`|ExecutionSequence`
    (:`then_0`
      (`ActorComponent.SetIsReplicated` (`self.Sprite`) true))
    (:`then_1`
      (bind _returnvalue (`|CreateWidget` "/Game/GameOfSam/BP/Widget_HUD.Widget_HUD_C" (`GameplayStatics.GetPlayerController` 0)))
      (bind _output_get (set `self.HealthBar` _returnvalue))
      (`UserWidget.AddToViewport` _output_get 0))))

(event `UpdateAnimation`
  (bind _sprite (`self.Sprite`))
  ;[1 1 1] Handle Animation
  (switch `/Game/GameOfSam/BP/State` (`self.CharacterState`)
    (:`NewEnumerator0`
      (`PaperFlipbookComponent.SetFlipbook` _sprite (select `bool` (> (`KismetMathLibrary.VSize` (`self.GetVelocity`)) 0.0) :`false` "/Game/GameOfSam/Sprites/Player/Anim_Idle.Anim_Idle" :`true` "/Game/GameOfSam/Sprites/Player/Anim_Run.Anim_Run" :!type "PaperFlipbook Object Reference")))
    (:`NewEnumerator2`
      (`PaperFlipbookComponent.SetFlipbook` _sprite "/Game/GameOfSam/Sprites/Player/Anim_Jump.Anim_Jump"))
    (:`NewEnumerator5`
      (`PaperFlipbookComponent.SetFlipbook` _sprite "/Game/GameOfSam/Sprites/Player/Anim_Dead.Anim_Dead"))
    (:`NewEnumerator6`
      (`PaperFlipbookComponent.SetFlipbook` _sprite "/Game/GameOfSam/Sprites/Player/Anim_ShootingInAir.Anim_ShootingInAir"))
    (:`NewEnumerator7`
      (`PaperFlipbookComponent.SetFlipbook` _sprite "/Game/GameOfSam/Sprites/Player/Anim_JumpingAfterShooting.Anim_JumpingAfterShooting"))))

(event `InputAxis|MoveRight`
  (params (AxisValue :type "Float (single-precision)"))
  ;[1 1 1] Handle movement
  (if (> AxisValue 0.0)
    (set `self.isMovingRight` true)
    (elif (< AxisValue 0.0)
      (set `self.isMovingRight` false)))
  (`self.AddMovementInput` (1.0 0.0 0.0) AxisValue))

(event `self.ReceiveTick`
  (params (DeltaSeconds :type "Float (single-precision)"))
  (bind _returnvalue (`self.GetController`))
  (bind _returnvalue_2 (`self.GetController`))
  ;[1 1 1] Tick - Updates animation
  (`self.UpdateAnimation`)
  (`/Engine/EditorBlueprintResources/StandardMacros.CompareFloat` (.x (`MovementComponent.Velocity` (`self.GetMovementComponent`)))
    (:`>`
      (`/Engine/EditorBlueprintResources/StandardMacros.IsValid` _returnvalue_2 :!label _label_2
        (:`Is Valid`
          (`Controller.SetControlRotation` _returnvalue_2 (`KismetMathLibrary.MakeRotator` 0.0))
          (set `self.Facing` 1))))
    (:`==`
      (if (`self.isMovingRight`)
        (goto _label_2)
        (else
          (`/Engine/EditorBlueprintResources/StandardMacros.IsValid` _returnvalue :!label _label_3
            (:`Is Valid`
              (`Controller.SetControlRotation` _returnvalue (`KismetMathLibrary.MakeRotator` 0.0 0.0 180.0))
              (set `self.Facing` -1))))))
    (:`<`
      (goto _label_3))))

(event `ShotDestroyed`
  ;[1 1 1] Shoot
  (`/Engine/EditorBlueprintResources/StandardMacros.DecrementInt` (`self.ShotsAlive`)
    (:`  `
      (if (`PlayerController.IsInputKeyDown` (`GameplayStatics.GetPlayerController` 0) (stale `InputAction|Shoot` Key)) :!label _label_4
        (`self.Shoot`)))))

(event `InputAction|Jump`
  (params (Key :type "Key Structure"))
  ;[1 1 1] Handle Jump
  (:`Pressed`
    (`self.Jump` :!label _label_5)
    (set `self.CharacterState` "NewEnumerator2"))
  (:`Released`
    (`self.StopJumping` :!label _label_6)))

(event `Shoot`
  ;[1 1 1] Shoot
  (if (and (not (`self.ShotRecently`)) (< (`self.ShotsAlive`) (`self.MaxShots`)))
    (set `self.ShotRecently` true)
    (`|ExecutionSequence`
      (:`then_0`
        (`KismetSystemLibrary.Delay` (`self.ShotDelay`))
        (set `self.ShotRecently` false)
        (goto _label_4))
      (:`then_1`
        (if (or (`|EnumEquality` "NewEnumerator2" (`self.CharacterState`)) (`|EnumEquality` "NewEnumerator6" (`self.CharacterState`)) (`|EnumEquality` "NewEnumerator7" (`self.CharacterState`)))
          (`|ExecutionSequence`
            (:`then_0`
              (bind _returnvalue (`|SpawnActorFromClass` "/Game/GameOfSam/BP/BP_Shot.BP_Shot_C" (`SceneComponent.K2_GetComponentToWorld` (`self.Arrow1`)) "Undefined" "OverrideRootScale" null null))
              (`/Game/GameOfSam/BP/BP_Shot.ShootDown` _returnvalue)
              (`/Engine/EditorBlueprintResources/StandardMacros.IncrementInt` (`self.ShotsAlive`)
                (:`  `
                  (set `MovementComponent.Velocity` (0.0 0.0 0.0) (`self.CharacterMovement`)))))
            (:`then_1`
              (`self.LaunchCharacter` (`self.ShotKnockback`))
              (set `self.CharacterState` "NewEnumerator6")
              (`self.UpdateAnimation`)
              (`KismetSystemLibrary.Delay` 0.2)
              (if (not (`PlayerController.IsInputKeyDown` (`GameplayStatics.GetPlayerController` 0) (stale `InputAction|Shoot` Key)))
                (set `self.CharacterState` "NewEnumerator7")
                (`self.UpdateAnimation`))))
          (else
            (`|SpawnActorFromClass` "/Game/GameOfSam/BP/BP_Shot.BP_Shot_C" (`SceneComponent.K2_GetComponentToWorld` (`self.Arrow1`)) "Undefined" "OverrideRootScale" null null)
            (`/Engine/EditorBlueprintResources/StandardMacros.IncrementInt` (`self.ShotsAlive`)))))
      (:`then_2`
        (`KismetSystemLibrary.PrintString` (`KismetStringLibrary.Conv_IntToString` (`self.ShotsAlive`)))))))

(event `InputTouch`
  (params (Location :type "Vector Structure") (FingerIndex :type "ETouchIndex Enum"))
  ;[1 1 1] Handle Jump
  (:`Pressed`
    (goto _label_5))
  (:`Released`
    (goto _label_6)))

(event `self.OnLanded`
  (params (Hit :type "HitResult Structure (by ref)"))
  ;[1 1 1] Handle Jump
  (set `self.CharacterState` "NewEnumerator0")
  (`self.EnableInput` (`GameplayStatics.GetPlayerController` 0)))

(event `InputAction|Shoot`
  (params (Key :type "Key Structure"))
  ;[1 1 1] Shoot
  (:`Pressed`
    (`self.Shoot`)))

(fn `UserConstructionScript`)